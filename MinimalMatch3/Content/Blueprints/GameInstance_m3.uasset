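; Game instance for the m3 tile game that holds player settings and game options, persists them in a save slot, and manages music.
; StartUp loads the save or creates defaults, applies sound-mix volumes and frame-rate/VSync settings, then shows a splash leading to the main menu, or to settings on first play.
; SaveCurrentValues writes the variables back and reapplies audio and video settings.
; MusicPlay swaps the 2D track only when it changes.
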(event Custom|StartUp
  (bind _savegamename (Variables|SaveGame|GetSaveGameName))
  ;[0 1 0] Start Up Checks
  ;[1 0.2462 0.3863] Check for Save Game (Either Load Existing or Create New)
  (bind _returnvalue (SaveGame|DoesSaveGameExist _savegamename))
  (if _returnvalue
    (bind _returnvalue_2 (SaveGame|LoadGamefromSlot _savegamename))
    (bind _asm_3save_game (Utilities|Casting|CastTom3SaveGame _returnvalue_2)
      (:then
        ;[0.9635 0.9635 0.9635] Get/Set LightMode? Setting
        (Variables|Settings|SetLightMode? (Variables|/Game/Blueprints/m3SaveGame.m3SaveGame_C|GetLightMode? _asm_3save_game))
        ;[0.9635 0.9635 0.9635] Get/Set AccentColor Setting
        (Variables|Settings|SetAccentColor (Variables|/Game/Blueprints/m3SaveGame.m3SaveGame_C|GetAccentColor _asm_3save_game))
        ;[0.9635 0.9635 0.9635] Get/Set AudioMuted? Setting
        (Variables|Settings|SetAudioMuted? (Variables|/Game/Blueprints/m3SaveGame.m3SaveGame_C|GetAudioMuted? _asm_3save_game))
        ;[0.9635 0.9635 0.9635] Get/Set AudioSFX Volume
        (Variables|Settings|SetAudioSFX (Variables|/Game/Blueprints/m3SaveGame.m3SaveGame_C|GetAudioSFX _asm_3save_game))
        ;[0.9635 0.9635 0.9635] Get/Set AudioMusic Volume Setting
        (Variables|Settings|SetAudioMusic (Variables|/Game/Blueprints/m3SaveGame.m3SaveGame_C|GetAudioMusic _asm_3save_game))
        ;[0.9635 0.9635 0.9635] Get/Set AudioAmbient Volume Setting
        (Variables|Settings|SetAudioAmbient (Variables|/Game/Blueprints/m3SaveGame.m3SaveGame_C|GetAudioAmbient _asm_3save_game))
        ;[0.9531 0.9531 0.9531] Get/Set Audio Volumes
        (if (Variables|Settings|GetAudioMuted?)
          (Class|GameplayStatics|SetBaseSoundMix "/Game/Audio/A_Mix_Mute.A_Mix_Mute")
          (Audio|SetSoundMixClassOverride "/Game/Audio/A_Mix_Mute.A_Mix_Mute" "/Game/Audio/A_SoundClass_SFX.A_SoundClass_SFX" 1e-06 1.0 0.0 true)
          (Audio|SetSoundMixClassOverride "/Game/Audio/A_Mix_Mute.A_Mix_Mute" "/Game/Audio/A_SoundClass_Music.A_SoundClass_Music" 1e-06 1.0 0.0 true)
          (Audio|SetSoundMixClassOverride "/Game/Audio/A_Mix_Mute.A_Mix_Mute" "/Game/Audio/A_SoundClass_Ambient.A_SoundClass_Ambient" 1e-06 1.0 0.0 true)
          (else
            (Class|GameplayStatics|SetBaseSoundMix "/Game/Audio/A_Mix_Default.A_Mix_Default")
            (Audio|SetSoundMixClassOverride "/Game/Audio/A_Mix_Default.A_Mix_Default" "/Game/Audio/A_SoundClass_SFX.A_SoundClass_SFX" (Variables|Settings|GetAudioSFX) 1.0 0.0 true)
            (Audio|SetSoundMixClassOverride "/Game/Audio/A_Mix_Default.A_Mix_Default" "/Game/Audio/A_SoundClass_Music.A_SoundClass_Music" (Variables|Settings|GetAudioMusic) 1.0 0.0 true)
            (Audio|SetSoundMixClassOverride "/Game/Audio/A_Mix_Default.A_Mix_Default" "/Game/Audio/A_SoundClass_Ambient.A_SoundClass_Ambient" (Variables|Settings|GetAudioAmbient) 1.0 0.0 true)))
        ;[0.9427 0.9427 0.9427] Get/Set User Settings (Save/Apply FrameRateLimit and VSync)
        (bind _returnvalue_3 (Settings|GetGameUserSettings))
        (bind _output_get (Variables|Settings|SetVideoFrameRateLimit (Variables|/Game/Blueprints/m3SaveGame.m3SaveGame_C|GetVideoFrameRateLimit _asm_3save_game)))
        (Class|GameUserSettings|SetFrameRateLimit _returnvalue_3 _output_get)
        (bind _output_get_2 (Variables|Settings|SetVSync? (Variables|/Game/Blueprints/m3SaveGame.m3SaveGame_C|GetVSync? _asm_3save_game)))
        (Class|GameUserSettings|SetVSyncEnabled _returnvalue_3 _output_get_2)
        (Class|GameUserSettings|ApplySettings _returnvalue_3 true)
        (Class|GameUserSettings|SaveSettings _returnvalue_3)
        ;[0.9635 0.9635 0.9635] Get/Set GameMode Game Option
        (Variables|Gameplay|SetGameMode (Variables|/Game/Blueprints/m3SaveGame.m3SaveGame_C|GetGameMode _asm_3save_game))
        ;[0.9635 0.9635 0.9635] Get/Set RowCount Game Option
        (Variables|Gameplay|SetTileRowCount (Variables|/Game/Blueprints/m3SaveGame.m3SaveGame_C|GetTileRowCount _asm_3save_game))
        ;[0.9635 0.9635 0.9635] Get/Set ColumnCount Game Option
        (Variables|Gameplay|SetTileColumnCount (Variables|/Game/Blueprints/m3SaveGame.m3SaveGame_C|GetTileColumnCount _asm_3save_game))
        ;[0 1 0.25] Create Widget - Existing Player: Splash, then Main Menu
        (bind _returnvalue_4 (UserInterface|CreateWidget "/Game/Widgets/WBP_Splash.WBP_Splash_C"))
        (UserInterface|Viewport|AddtoViewport _returnvalue_4 0)
        (Variables|/Game/Widgets/WBP_Splash.WBP_Splash_C|SetNextWidget _returnvalue_4 "/Game/Widgets/WBP_Menu-Main.WBP_Menu-Main_C"))
      (:CastFailed
        (bind _returnvalue_5 (SaveGame|CreateSaveGameObject (Variables|SaveGame|GetSaveGameClass) :!label _label))
        (SaveGame|SaveGametoSlot _returnvalue_5 _savegamename)
        ;[0.9635 0.9635 0.9635] Set LightMode? Setting
        (Variables|Settings|SetLightMode? false)
        ;[0.9635 0.9635 0.9635] Set AccentColor Setting
        (Variables|Settings|SetAccentColor "(R=0.500000,G=0.500000,B=0.500000,A=1.000000)")
        ;[0.9635 0.9635 0.9635] Set AudioMuted? Setting
        (Variables|Settings|SetAudioMuted? false)
        ;[0.9635 0.9635 0.9635] Set AudioSFX Volume Setting
        (Variables|Settings|SetAudioSFX 1.0)
        ;[0.9635 0.9635 0.9635] Set AudioMusic Volume Setting
        (Variables|Settings|SetAudioMusic 1.0)
        ;[0.9635 0.9635 0.9635] Set AudioAmbient Volume Setting
        (Variables|Settings|SetAudioAmbient 1.0)
        (Class|GameplayStatics|SetBaseSoundMix "/Game/Audio/A_Mix_Default.A_Mix_Default")
        (Audio|SetSoundMixClassOverride "/Game/Audio/A_Mix_Default.A_Mix_Default" "/Game/Audio/A_SoundClass_SFX.A_SoundClass_SFX" (Variables|Settings|GetAudioSFX) 1.0 0.0 true)
        (Audio|SetSoundMixClassOverride "/Game/Audio/A_Mix_Default.A_Mix_Default" "/Game/Audio/A_SoundClass_Music.A_SoundClass_Music" (Variables|Settings|GetAudioMusic) 1.0 0.0 true)
        (Audio|SetSoundMixClassOverride "/Game/Audio/A_Mix_Default.A_Mix_Default" "/Game/Audio/A_SoundClass_Ambient.A_SoundClass_Ambient" (Variables|Settings|GetAudioAmbient) 1.0 0.0 true)
        ;[0.9427 0.9427 0.9427] Get/Set User Settings (Save/Apply FrameRateLimit and VSync)
        (bind _returnvalue_6 (Settings|GetGameUserSettings))
        (Class|GameUserSettings|ApplySettings _returnvalue_6 true)
        (Variables|Settings|SetVideoFrameRateLimit (Class|GameUserSettings|GetFrameRateLimit _returnvalue_6))
        (Variables|Settings|SetVSync? (Class|GameUserSettings|IsVSyncEnabled _returnvalue_6))
        (Class|GameUserSettings|SaveSettings _returnvalue_6)
        ;[0.9635 0.9635 0.9635] Set GameMode Game Option
        (Variables|Gameplay|SetGameMode "Choose")
        ;[0.9635 0.9635 0.9635] Set RowCount Game Option
        (Variables|Gameplay|SetTileRowCount 3)
        ;[0.9635 0.9635 0.9635] Set ColumnCount Game Option
        (Variables|Gameplay|SetTileColumnCount 3)
        (Utilities|FlowControl|Sequence
          (:then_0
            ;[0 1 0.25] Create Widget - First Play: Splash, then Menu-Settings, then Menu-Color, then Main Menu
            (bind _returnvalue_7 (UserInterface|CreateWidget "/Game/Widgets/WBP_Splash.WBP_Splash_C"))
            (UserInterface|Viewport|AddtoViewport _returnvalue_7 0)
            (Variables|/Game/Widgets/WBP_Splash.WBP_Splash_C|SetNextWidget _returnvalue_7 "/Game/Widgets/WBP_Menu-Settings.WBP_Menu-Settings_C"))
          (:then_1
            ;[1 0.2462 0.3863] Save Game with Current Values
            (CallFunction|SaveCurrentValues)))))
    (else
      (goto _label))))

(event Custom|MusicStop
  (bind _sound_music_component (Variables|Audio|GetSound_Music-Component))
  ;[0.25 0 1] Stop Music
  (Utilities|IsValid _sound_music_component
    (:Is%20Valid
      (Audio|Components|Audio|Stop _sound_music_component)
      (Components|DestroyComponent _sound_music_component))))

(event Custom|MusicPlay
  (params (SoundBase :type Sound%20Base%20Object%20Reference))
  ;[0.25 0 1] Play Music
  (Utilities|IsValid SoundBase
    (:Is%20Valid
      (Utilities|IsValid (Variables|Audio|GetSound_Music)
        (:Is%20Valid
          (if (not (== SoundBase (Variables|Audio|GetSound_Music)))
            (Utilities|FlowControl|Sequence :!label _label
              (:then_0
                (CallFunction|MusicStop))
              (:then_1
                (bind _output_get (Variables|Audio|SetSound_Music SoundBase))
                (bind _returnvalue (Audio|SpawnSound2D _output_get 1.0 1.0 0.0 0))
                (Variables|Audio|SetSound_Music-Component _returnvalue)))))
        (:Is%20Not%20Valid
          (goto _label))))))

(event Custom|SaveCurrentValues
  (bind _savegamename (Variables|SaveGame|GetSaveGameName))
  ;[1 0.2462 0.3863] Save Game with Current Values
  ;[1 0.2462 0.3863] Save Game with Current Values
  (bind _returnvalue (SaveGame|DoesSaveGameExist _savegamename))
  (if _returnvalue
    (bind _returnvalue_2 (SaveGame|LoadGamefromSlot _savegamename))
    (bind _asm_3save_game (Utilities|Casting|CastTom3SaveGame _returnvalue_2)
      (:then
        ;[0.9635 0.9635 0.9635] Set LightMode? Setting
        (Variables|/Game/Blueprints/m3SaveGame.m3SaveGame_C|SetLightMode? _asm_3save_game (Variables|Settings|GetLightMode?))
        ;[0.9635 0.9635 0.9635] Set AccentColor Setting
        (Variables|/Game/Blueprints/m3SaveGame.m3SaveGame_C|SetAccentColor _asm_3save_game (Variables|Settings|GetAccentColor))
        ;[0.9635 0.9635 0.9635] Set AudioMuted? Setting
        (Variables|/Game/Blueprints/m3SaveGame.m3SaveGame_C|SetAudioMuted? _asm_3save_game (Variables|Settings|GetAudioMuted?))
        ;[0.9635 0.9635 0.9635] Set AudioSFX Volume Setting
        (Variables|/Game/Blueprints/m3SaveGame.m3SaveGame_C|SetAudioSFX _asm_3save_game (Variables|Settings|GetAudioSFX))
        ;[0.9635 0.9635 0.9635] Set AudioMusic Volume Setting
        (Variables|/Game/Blueprints/m3SaveGame.m3SaveGame_C|SetAudioMusic _asm_3save_game (Variables|Settings|GetAudioMusic))
        ;[0.9635 0.9635 0.9635] Set AudioAmbient Volume Setting
        (Variables|/Game/Blueprints/m3SaveGame.m3SaveGame_C|SetAudioAmbient _asm_3save_game (Variables|Settings|GetAudioAmbient))
        ;[0.9635 0.9635 0.9635] Set Video Frame Rate Limit Setting
        (Variables|/Game/Blueprints/m3SaveGame.m3SaveGame_C|SetVideoFrameRateLimit _asm_3save_game (Variables|Settings|GetVideoFrameRateLimit))
        ;[0.9635 0.9635 0.9635] Set Video Frame Rate Limit Setting
        (Variables|/Game/Blueprints/m3SaveGame.m3SaveGame_C|SetVSync? _asm_3save_game (Variables|Settings|GetVSync?))
        ;[0.9635 0.9635 0.9635] Set GameMode Game Option
        (Variables|/Game/Blueprints/m3SaveGame.m3SaveGame_C|SetGameMode _asm_3save_game (Variables|Gameplay|GetGameMode))
        ;[0.9635 0.9635 0.9635] Set RowCount Game Option
        (Variables|/Game/Blueprints/m3SaveGame.m3SaveGame_C|SetTileRowCount _asm_3save_game (Variables|Gameplay|GetTileRowCount))
        ;[0.9635 0.9635 0.9635] Set ColumnCount Game Option
        (Variables|/Game/Blueprints/m3SaveGame.m3SaveGame_C|SetTileColumnCount _asm_3save_game (Variables|Gameplay|GetTileColumnCount))
        (SaveGame|SaveGametoSlot _asm_3save_game _savegamename)
        ;[0.9531 0.9531 0.9531] Get/Set Audio Volumes
        (if (Variables|Settings|GetAudioMuted?)
          (Class|GameplayStatics|SetBaseSoundMix "/Game/Audio/A_Mix_Mute.A_Mix_Mute")
          (Audio|SetSoundMixClassOverride "/Game/Audio/A_Mix_Mute.A_Mix_Mute" "/Game/Audio/A_SoundClass_SFX.A_SoundClass_SFX" 1e-06 1.0 0.0 true)
          (Audio|SetSoundMixClassOverride "/Game/Audio/A_Mix_Mute.A_Mix_Mute" "/Game/Audio/A_SoundClass_Music.A_SoundClass_Music" 1e-06 1.0 0.0 true)
          (Audio|SetSoundMixClassOverride "/Game/Audio/A_Mix_Mute.A_Mix_Mute" "/Game/Audio/A_SoundClass_Ambient.A_SoundClass_Ambient" 1e-06 1.0 0.0 true)
          (else
            (Class|GameplayStatics|SetBaseSoundMix "/Game/Audio/A_Mix_Default.A_Mix_Default" :!label _label)
            (Audio|SetSoundMixClassOverride "/Game/Audio/A_Mix_Default.A_Mix_Default" "/Game/Audio/A_SoundClass_SFX.A_SoundClass_SFX" (Variables|Settings|GetAudioSFX) 1.0 0.0 true)
            (Audio|SetSoundMixClassOverride "/Game/Audio/A_Mix_Default.A_Mix_Default" "/Game/Audio/A_SoundClass_Music.A_SoundClass_Music" (Variables|Settings|GetAudioMusic) 1.0 0.0 true)
            (Audio|SetSoundMixClassOverride "/Game/Audio/A_Mix_Default.A_Mix_Default" "/Game/Audio/A_SoundClass_Ambient.A_SoundClass_Ambient" (Variables|Settings|GetAudioAmbient) 1.0 0.0 true))))
      (:CastFailed
        (bind _returnvalue_3 (SaveGame|CreateSaveGameObject (Variables|SaveGame|GetSaveGameClass) :!label _label_2))
        (SaveGame|SaveGametoSlot _returnvalue_3 _savegamename)
        (goto _label)))
    (else
      (goto _label_2)))
  ;[0.9427 0.9427 0.9427] Get/Set User Settings (Save/Apply FrameRateLimit and VSync)
  (bind _returnvalue_4 (Settings|GetGameUserSettings))
  (Class|GameUserSettings|SetFrameRateLimit _returnvalue_4 (Variables|Settings|GetVideoFrameRateLimit))
  (Class|GameUserSettings|SetVSyncEnabled _returnvalue_4 (Variables|Settings|GetVSync?))
  (Class|GameUserSettings|ApplySettings _returnvalue_4 true)
  (Class|GameUserSettings|SaveSettings _returnvalue_4))