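; Game instance that owns the persistent light/dark mode setting and opens the splash screen.
; StartUp loads or creates the m3SaveGame slot, copies its LightMode (false if invalid) and adds the WBP_SplashDP widget to the viewport.
; ChangeLightMode updates the value and calls the save function, which writes it into an existing save.
; If that save is missing or fails its cast, it saves a new object without copying LightMode.
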(event Custom|StartUp
  ;[0 1 0] Start Up Checks
  ;[1 0.2462 0.3863] Check for Save Game (Either Load Existing or Create New)
  (bind _m3savegame (CallFunction|FunctionCheckforSaveGame))
  (Utilities|IsValid _m3savegame
    (:Is%20Valid
      ;[0.9635 0.9635 0.9635] Get/Set LightMode? Setting
      (Variables|Settings|SetLightMode? (Variables|/Game/Blueprints/m3SaveGame.m3SaveGame_C|GetLightMode? _m3savegame)))
    (:Is%20Not%20Valid
      ;[0.9635 0.9635 0.9635] Set LightMode? Setting
      (Variables|Settings|SetLightMode? false)))
  ;[0 1 0.25] Create Widget - Splash-DP
  (bind _returnvalue (UserInterface|CreateWidget "/Game/Widgets/WBP_Splash-DP.WBP_Splash-DP_C"))
  (UserInterface|Viewport|AddtoViewport _returnvalue 0))

(event Custom|ChangeLightMode
  (params (LightMode? :type Boolean))
  ;[0.9635 0.9635 0.9635] Change between Dark Mode and Light Mode
  (Variables|Settings|SetLightMode? LightMode?)
  ;[1 0.2462 0.3863] Save Game with Current Values
  (CallFunction|FunctionSaveGame))

(fn FunctionCheckforSaveGame
  ;[1 0.2462 0.3863] Check for Save Game (Either Load Existing or Create New)
  (bind _returnvalue (SaveGame|DoesSaveGameExist "m3SaveGame"))
  (if _returnvalue
    (bind _returnvalue_2 (SaveGame|LoadGamefromSlot "m3SaveGame"))
    (bind _asm_3save_game (Utilities|Casting|CastTom3SaveGame _returnvalue_2)
      (:then
        (return _asm_3save_game))
      (:CastFailed
        _)))
  (bind _returnvalue_3 (SaveGame|CreateSaveGameObject "/Game/Blueprints/m3SaveGame.m3SaveGame_C"))
  (SaveGame|SaveGametoSlot _returnvalue_3 "m3SaveGame")
  (return _returnvalue_3))

(fn FunctionSaveGame
  ;[1 0.2462 0.3863] Save Game with Current Values
  (bind _returnvalue (SaveGame|DoesSaveGameExist "m3SaveGame"))
  (if _returnvalue
    (bind _returnvalue_2 (SaveGame|LoadGamefromSlot "m3SaveGame"))
    (bind _asm_3save_game (Utilities|Casting|CastTom3SaveGame _returnvalue_2)
      (:then
        (Variables|/Game/Blueprints/m3SaveGame.m3SaveGame_C|SetLightMode? _asm_3save_game (Variables|Settings|GetLightMode?))
        (SaveGame|SaveGametoSlot _asm_3save_game "m3SaveGame")
        (return _asm_3save_game))
      (:CastFailed
        _)))
  (bind _returnvalue_3 (SaveGame|CreateSaveGameObject "/Game/Blueprints/m3SaveGame.m3SaveGame_C"))
  (SaveGame|SaveGametoSlot _returnvalue_3 "m3SaveGame")
  (return _returnvalue_3))